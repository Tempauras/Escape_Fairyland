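; BP_Firewall is a wall of fire that hurts the player on contact and is put out by water bullets.
; On begin play it creates a dynamic material instance and starts two fire sounds.
; A water bullet hit toggles those sounds, then a timeline drives the material's Strength before an extinguish sound plays and the actor is destroyed.
; A player hit applies contact damage and launches the character along world Y.
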(event OnComponentHit(StaticMeshComponent)
  (params (HitComponent :type Primitive%20Component%20Object%20Reference) (OtherActor :type Actor%20Object%20Reference) (OtherComp :type Primitive%20Component%20Object%20Reference) (NormalImpulse :type Vector :default "0, 0, 0") (Hit :type Hit%20Result%20Structure%20%28by%20ref%29))
  (bind _returnvalue (Utilities|GetClass OtherActor))
  (Utilities|FlowControl|Delay 0.1)
  (if (== _returnvalue "/Game/Blueprints/ElementalGun/BP/WaterBullet.WaterBullet_C")
    (Components|Activation|ToggleActive (stale EventBeginPlay _returnvalue_3))
    (Components|Activation|ToggleActive (stale EventBeginPlay _returnvalue_4))
    (bind _firewall_disappearing_track (Timeline|Timeline_0 Play)
      (:Update
        (Rendering|Material|SetScalarParameterValue (Variables|Default|GetMI_FireWall) "Strength" _firewall_disappearing_track :!class /Script/Engine.MaterialInstanceDynamic))
      (:Finished
        (Audio|PlaySoundatLocation "/Game/ThirdParty/Sounds/SoundEffect/Fire_Extinguished_Cue.Fire_Extinguished_Cue" (Transformation|GetActorLocation) "0, 0, 0" 1.0 1.0 0.0 0 0 0)
        (Actor|DestroyActor)))
    (elif (== _returnvalue "/Game/FirstPersonBP/Blueprints/FirstPersonCharacter.FirstPersonCharacter_C")
      (bind _asfirst_person_character (Utilities|Casting|CastToFirstPersonCharacter OtherActor))
      (Default|UpdateLife _asfirst_person_character (Variables|Default|GetcontactDamage))
      (Character|LaunchCharacter _asfirst_person_character "0,5000.000000, 0" false false))))

(event EventBeginPlay
  (bind _returnvalue (Transformation|GetActorLocation))
  (bind _staticmeshcomponent (Variables|Debug|GetStaticMeshComponent))
  (bind _returnvalue_2 (Rendering|Material|CreateDynamicMaterialInstance _staticmeshcomponent 0 (Rendering|Material|GetMaterial _staticmeshcomponent 0) "None" :!class /Script/Engine.PrimitiveComponent))
  (Variables|Default|SetMI_FireWall _returnvalue_2)
  (bind _returnvalue_3 (Audio|SpawnSoundatLocation "/Game/ThirdParty/Sounds/SoundEffect/Fire1_Cue.Fire1_Cue" _returnvalue "0, 0, 0" 1.0 1.0 0.0 0 0))
  (bind _returnvalue_4 (Audio|SpawnSoundatLocation "/Game/ThirdParty/Sounds/SoundEffect/Fire2_Cue.Fire2_Cue" _returnvalue "0, 0, 0" 1.0 1.0 0.0 0 0)))

(fn ConstructionScript)