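; BP_ChewingGum is a charge-and-fire chewing gum tool that temporarily switches off collision on the component it hits.
; While charging, Tick reads left-mouse hold time; on release, only a full charge extends the effect duration before calling Shoot.
; Shoot uses ammo on a camera-forward visibility trace hit, sets NoCollision, then after a Delay sets BlockAll, refunds the ammo and resets the duration.
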(event EventTick
  (params (DeltaSeconds :type Float%20%28single-precision%29))
  (if (Variables|Default|GetisCharging)
    (Development|PrintString "charging")
    (bind _output_get (Variables|Default|Setcharge (Class|PlayerController|GetInputKeyTimeDown (Game|GetPlayerController 0) "LeftMouseButton")))
    (Development|PrintString (Utilities|String|ToString(Float) _output_get))))

(event EventCharging
  (Variables|Default|SetisCharging true))

(event EventReleasing
  (bind _maxcharge (Variables|Default|GetmaxCharge))
  (Variables|Default|SetisCharging false)
  (if (>= (Variables|Default|Getcharge) _maxcharge)
    (bind _output_get (Variables|Default|Setcharge _maxcharge))
    (Variables|Default|SetcurrPowerTime (+ _output_get (Variables|Default|GetcurrPowerTime))))
  (CallFunction|Shoot))

(event EventShoot
  (bind _returnvalue (Game|GetPlayerCameraManager 0))
  (bind _returnvalue_2 (Transformation|GetActorLocation _returnvalue))
  (if (> (Variables|Default|Getammo) 0)
    (bind (_outhit _returnvalue_3) (Collision|LineTraceByChannel _returnvalue_2 (+ _returnvalue_2 (* (Transformation|GetActorForwardVector _returnvalue) 5e+03)) "TraceTypeQuery1" false 0 "ForDuration" false))
    (if _returnvalue_3
      (Variables|Default|Setammo (+ (Variables|Default|Getammo) -1))
      (bind _output_get (Variables|Default|SetHit%20Component (.HitComponent (Collision|BreakHitResult _outhit))))
      (Development|PrintString (Utilities|GetDisplayName _output_get))
      (Collision|SetCollisionProfileName _output_get "NoCollision" true :!class /Script/Engine.PrimitiveComponent)
      (Utilities|FlowControl|Delay (Variables|Default|GetcurrPowerTime))
      (Development|PrintString (Utilities|GetDisplayName (Variables|Default|GetHit%20Component)))
      (Collision|SetCollisionProfileName (Variables|Default|GetHit%20Component) "BlockAll" true :!class /Script/Engine.PrimitiveComponent)
      (Variables|Default|Setammo (+ (Variables|Default|Getammo) 1))
      (Variables|Default|SetcurrPowerTime (Variables|Default|GetpowerTime)))
    (else
      (Development|PrintString "NoAmmo"))))

(fn ConstructionScript
  (|CallParentFunction))