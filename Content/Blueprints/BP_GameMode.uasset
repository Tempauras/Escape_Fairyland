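; Game mode Blueprint that handles checkpoint respawning and game over.
; On BeginPlay it caches the first player's pawn as PlayerCharacter.
; RespawnPlayer moves that pawn to LastCheckPoint and sets the controller rotation from the checkpoint's Arrow forward vector.
; GameOver prints a message, waits briefly, then opens MainLevel.
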(event Custom|RespawnPlayer
  (Transformation|SetActorLocation (Variables|Default|GetplayerCharacter) (Transformation|GetActorLocation (Variables|Default|GetlastCheckPoint)) false false)
  (Pawn|SetControlRotation (Game|GetPlayerController 0) (Math|Rotator|MakeRotfromXY (Math|Vector|GetForwardVector (Variables|/Game/Blueprints/BP_checkpoint.BP_checkpoint_C|GetArrow (Variables|Default|GetlastCheckPoint))) (Math|Vector|MakeVector 0.0 0.0 0.0))))

(event Custom|RegisterPlayer
  (Variables|Default|SetplayerCharacter (Game|Player|GetPlayerPawn 0)))

(event Custom|GameOver
  (Development|PrintString "GAMEOVER")
  (Utilities|FlowControl|Delay 1.0)
  (Game|OpenLevel(byName) "MainLevel"))

(event EventBeginPlay
  (CallFunction|RegisterPlayer))

(event EventTick
  (params (DeltaSeconds :type Float%20%28single-precision%29)))

(fn ConstructionScript)