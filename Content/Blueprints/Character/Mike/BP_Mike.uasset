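; BP_Mike is a character Blueprint that leaves a tag-dependent object at its start position when it dies.
; BeginPlay sets life and records the spawn transform, then flags death after a three-second delay; CheckLife also flags it at zero life.
; Tick calls Dead, which spawns a lowered weapon spawner granting the elemental gun for "SpawnMike" or a button for "1stPartMike", then destroys the actor.
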(event Custom|CheckLife
  (if (<= (Variables|Default|GetcurrentLife) 0.0)
    (Variables|Default|SetisDead true)))

(event Custom|Dead
  (bind _spawnposition (Variables|Default|GetSpawnPosition))
  (bind _spawnposition_2 (Variables|Default|GetSpawnPosition))
  (if (Actor|ActorHasTag "SpawnMike")
    (bind _returnvalue (Game|SpawnActorfromClass "/Game/Buginatron/SpawnWeapon.SpawnWeapon_C" (Math|Transform|MakeTransform (Math|Vector|MakeVector (.x (.location _spawnposition_2)) (.y (.location _spawnposition_2)) (- (.z (.location _spawnposition_2)) 75.0)) (.rotation _spawnposition_2) (.scale _spawnposition_2)) "Undefined" 0 0))
    (Variables|/Game/Buginatron/SpawnWeapon.SpawnWeapon_C|Setweapon _returnvalue "/Game/Blueprints/ElementalGun/BP/BP_ElementalGun.BP_ElementalGun_C")
    (Default|ForceAddWeapon _returnvalue)
    (Actor|DestroyActor)
    (elif (Actor|ActorHasTag "1stPartMike")
      (Game|SpawnActorfromClass "/Game/Blueprints/BP_Button.BP_Button_C" (Math|Transform|MakeTransform (Math|Vector|MakeVector (.x (.location _spawnposition)) (.y (.location _spawnposition)) (- (.z (.location _spawnposition)) 75.0)) (.rotation _spawnposition) (.scale _spawnposition)) "Undefined" 0 (Game|Player|GetPlayerPawn 0))
      (Actor|DestroyActor))))

(event EventTick
  (params (DeltaSeconds :type Float%20%28single-precision%29))
  (if (Variables|Default|GetisDead)
    (CallFunction|Dead)))

(event EventBeginPlay
  (Variables|Default|SetisDead false)
  (bind _output_get (Variables|Default|SetmaxLife 3e+01))
  (Variables|Default|SetcurrentLife _output_get)
  (Variables|Default|SetSpawnPosition (Transformation|GetActorTransform))
  (Utilities|FlowControl|Delay 3.0)
  (Variables|Default|SetisDead true))

(fn ConstructionScript)