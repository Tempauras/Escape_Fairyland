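; Game mode that handles level progression and checkpoint respawning for the first-person player.
; On BeginPlay it fires the player-respawned dispatcher and caches the player pawn.
; NextLevel increments the GameInstance's level index and opens the map named by swapping the current name's last character for that index, until the final level.
; GameOver waits briefly, moves the player to the last checkpoint, aligns the view to its arrow and restores life.
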(event Custom|RespawnPlayer
  (Transformation|SetActorLocation (Variables|Default|GetplayerCharacter) (Transformation|GetActorLocation (Variables|Default|GetlastCheckPoint)) false false)
  (Pawn|SetControlRotation (Game|GetPlayerController 0) (Math|Rotator|MakeRotfromXY (Math|Vector|GetForwardVector (Variables|/Game/Blueprints/Props/BP_checkpoint.BP_checkpoint_C|GetArrow (Variables|Default|GetlastCheckPoint))) (Math|Vector|MakeVector 0.0 0.0 0.0))))

(event Custom|RegisterPlayer
  (Default|CallEDPlayerRespawned)
  (Variables|Default|SetplayerCharacter (Game|Player|GetPlayerPawn 0)))

(event Custom|GameOver
  (Development|PrintString "GAMEOVER")
  (Utilities|FlowControl|Delay 1.0)
  (CallFunction|RespawnPlayer)
  (bind _asfirst_person_character (Utilities|Casting|CastToFirstPersonCharacter (Variables|Default|GetplayerCharacter)))
  (Default|UpdateLife _asfirst_person_character 1e+02))

(event Custom|NextLevel
  (Development|PrintString "NEXTLEVEL")
  (bind _asbp_game_instance (Utilities|Casting|CastToBP_GameInstance (Game|GetGameInstance)))
  (if (< (+ (Variables|/Game/Blueprints/GameMode/BP_GameInstance.BP_GameInstance_C|GetindexCurrentLevel _asbp_game_instance) 1) 4)
    (bind _output_get (Variables|/Game/Blueprints/GameMode/BP_GameInstance.BP_GameInstance_C|SetindexCurrentLevel _asbp_game_instance (+ (Variables|/Game/Blueprints/GameMode/BP_GameInstance.BP_GameInstance_C|GetindexCurrentLevel _asbp_game_instance) 1)))
    (bind _returnvalue (Game|GetCurrentLevelName true))
    (Development|PrintString (Utilities|String|Append (Utilities|String|GetSubstring _returnvalue 0 (- (Utilities|String|Len _returnvalue) 1)) (Utilities|String|ToString(Integer) _output_get)))
    (Game|OpenLevel(byName) (Utilities|String|StringToName (Utilities|String|Append (Utilities|String|GetSubstring _returnvalue 0 (- (Utilities|String|Len _returnvalue) 1)) (Utilities|String|ToString(Integer) _output_get))))
    (bind _asfirst_person_character (Utilities|Casting|CastToFirstPersonCharacter (Variables|Default|GetplayerCharacter)))
    (Default|UpdateLife _asfirst_person_character 1e+02)
    (else
      (Development|PrintString "ENDGAME"))))

(event EventBeginPlay
  (CallFunction|RegisterPlayer))

(event EventTick
  (params (DeltaSeconds :type Float%20%28single-precision%29)))

(fn ConstructionScript)