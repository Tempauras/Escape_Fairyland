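; SecretCloudTest is a test Blueprint for a hidden element that appears temporarily when hit by the correct element.
; It starts hidden on BeginPlay, with Hide and Show events toggling its static mesh visibility and collision together.
; HitByCorrectElement shows it, loops the Level Sequence found through GetActorOfClass, then after a timed delay stops the sequence and hides the mesh again.
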(event Custom|HitByCorrectElement
  (CallFunction|Show)
  (bind _returnvalue (Actor|GetActorOfClass "/Script/LevelSequence.LevelSequenceActor"))
  (Class|MovieSceneSequencePlayer|PlayLooping (Variables|/Script/LevelSequence.LevelSequenceActor|GetSequencePlayer _returnvalue) 2)
  (Utilities|FlowControl|Delay (Variables|Default|GetTimer))
  (Sequencer|Player|Stop (Variables|/Script/LevelSequence.LevelSequenceActor|GetSequencePlayer _returnvalue) :!class /Script/MovieScene.MovieSceneSequencePlayer)
  (CallFunction|Hide))

(event Custom|Hide
  ;[1 1 1] Hide the Element
  (Rendering|SetVisibility (Variables|Debug|GetStaticMeshComponent) false false)
  (Collision|SetCollisionEnabled (Variables|Debug|GetStaticMeshComponent) "NoCollision"))

(event Custom|Show
  ;[1 1 1] Show the Element
  (Rendering|SetVisibility (Variables|Debug|GetStaticMeshComponent) true false)
  (Collision|SetCollisionEnabled (Variables|Debug|GetStaticMeshComponent) "QueryAndPhysics"))

(event EventBeginPlay
  (CallFunction|Hide)
  (Variables|Default|SetTimer 12.5))

(fn ConstructionScript)