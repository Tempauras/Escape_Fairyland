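; Base hitscan weapon with automatic fire, an overheat-style reload and its own HUD widget linked to the FirstPersonCharacter.
; A looping timer at FireRate traces from the muzzle socket toward the camera's aim point, spawning impact effects and applying radial damage on living BP_Cactus enemies.
; Heat works like ammo: each shot drains CurrHeat, and hitting zero triggers OverHeat, which blocks firing while a timeline refills it.
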(event Custom|activateUI
  (bind _returnvalue (UserInterface|CreateWidget "/Game/Blueprints/UI/WG_baseWeapon.WG_baseWeapon_C"))
  (UserInterface|Viewport|AddtoViewport _returnvalue 0)
  (bind _asfirst_person_character (Utilities|Casting|CastToFirstPersonCharacter (Game|GetPlayerCharacter 0)))
  (Variables|/Game/Blueprints/UI/WG_baseWeapon.WG_baseWeapon_C|Setplayer _returnvalue _asfirst_person_character))

(event Custom|OverHeat
  (Development|PrintString "Rechargement")
  (Variables|Default|SetisReloading true)
  (bind _heat (Timeline|TimelineReloadHeat PlayFromStart)
    (:Update
      (CallFunction|UpdateHeat _heat))
    (:Finished
      (Variables|Default|SetisReloading false))))

(event Custom|beginShooting
  (CallFunction|BaseWeaponShoot)
  (bind _returnvalue (Utilities|Time|SetTimerbyFunctionName 0 "Base Weapon Shoot" (Variables|Default|GetfireRate) true))
  (Variables|Default|SetgunTimer _returnvalue))

(event Custom|endShooting
  (Utilities|Time|ClearandInvalidateTimerbyHandle (Variables|Default|GetgunTimer)))

(fn ConstructionScript)

(fn BaseWeaponShoot
  (bind _returnvalue (Game|GetPlayerCameraManager 0))
  (if (> (Variables|Default|GetcurrHeat) 0.0)
    (if (Math|Boolean|Equal(Boolean) (Variables|Default|GetisReloading) false)
      (bind (_outhit _returnvalue_2) (Collision|LineTraceByChannel (Transformation|GetSocketLocation (Variables|Default|GetSkeletalMesh) "Ammo") (+ (Transformation|GetActorLocation _returnvalue) (* (Transformation|GetActorForwardVector _returnvalue) (Variables|Default|GetfireRange))) "TraceTypeQuery1" false 0 "None" true "(R=1.000000,G=0.000000,B=0.000000,A=1.000000)" "(R=0.000000,G=1.000000,B=0.000000,A=1.000000)" 1.0))
      (Audio|PlaySoundatLocation "/Game/FirstPerson/Audio/FirstPersonTemplateWeaponFire02.FirstPersonTemplateWeaponFire02" (Transformation|GetActorLocation) "0, 0, 0" 1.0 1.0 0.0 0 0 0)
      (CallFunction|UpdateHeat -1e+01)
      (if _returnvalue_2
        (if (== (Utilities|GetClass (.HitActor (Collision|BreakHitResult _outhit))) (Variables|Default|GetEnnemyClass))
          (Niagara|SpawnSystematLocation "/Game/ThirdParty/Stylized_VFX_StPack/Particles/P_Splash.P_Splash" (.Location (Collision|BreakHitResult _outhit)))
          (bind _asbp_cactus (Utilities|Casting|CastToBP_Cactus (.HitActor (Collision|BreakHitResult _outhit))))
          (if (Math|Boolean|NotEqual(Boolean) (Variables|/Game/Blueprints/Characters/Cactus/BP_Cactus.BP_Cactus_C|GetisDead _asbp_cactus) true)
            (Game|Damage|ApplyRadialDamage (Variables|Default|GetfireDamage) (.ImpactPoint (Collision|BreakHitResult _outhit)) (Variables|Default|GetfireDamageRadius) 0 0 0 0 false "ECC_Visibility"))
          (else
            (Niagara|SpawnSystematLocation "/Game/ThirdParty/Stylized_VFX_StPack/Particles/P_Hits.P_Hits" (.Location (Collision|BreakHitResult _outhit)))))))
    (else
      (CallFunction|OverHeat))))

(fn UpdateHeat
  (params (AddHeat :type Float%20%28single-precision%29))
  (bind _heat (Variables|Default|GetHeat))
  (if (<= (+ AddHeat (Variables|Default|GetcurrHeat)) 0.0)
    (Variables|Default|SetcurrHeat 0.0)
    (CallFunction|OverHeat)
    (elif (>= (+ AddHeat (Variables|Default|GetcurrHeat)) _heat)
      (Variables|Default|SetcurrHeat _heat)
      (else
        (Variables|Default|SetcurrHeat (+ AddHeat (Variables|Default|GetcurrHeat)))))))