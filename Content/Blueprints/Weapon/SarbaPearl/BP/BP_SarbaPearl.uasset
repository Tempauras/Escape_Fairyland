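; BP_SarbaPearl is a weapon that launches a BP_Cosmic_Projectile when shooting ends; BeginShooting does nothing.
; EndShooting checks Ammo, plays a laser cue at the mesh and spawns the gravity-enabled projectile just ahead of the Arrow component with a launch impulse.
; Ammo doubles as an anti-spam limiter: each shot decrements it, and a short Delay then refills it to MaxAmmo, which also seeds it on BeginPlay.
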(event EventBeginPlay
  (Variables|Default|SetAmmo (Variables|Default|GetmaxAmmo)))

(event EventBeginShooting)

(event EventEndShooting
  (bind _arrow (Variables|Default|GetArrow))
  (if (> (Variables|Default|GetAmmo) 0)
    ;[1 1 1] Play selected sound when the player shoot
    (Audio|PlaySoundatLocation "/Game/ThirdParty/Sounds/ArcadeShooter/SC_Laser_Cue.SC_Laser_Cue" (Transformation|GetWorldLocation (Variables|Default|GetSkeletalMesh)) "0, 0, 0" 1.0 1.0 0.0 0 0 0)
    ;[1 1 1] Create a projectile with a location and a rotation
    (Game|SpawnActorfromClass "/Game/Blueprints/Weapon/SarbaPearl/BP/BP_Cosmic_Projectile.BP_Cosmic_Projectile_C" (Math|Transform|MakeTransform (+ (Transformation|GetWorldLocation _arrow) (Math|Vector|GetForwardVector _arrow)) (Transformation|GetWorldRotation _arrow) "1,1,1") "AdjustIfPossibleButAlwaysSpawn" 0 true 4e+03 2 0)
    ;[1 1 1] Prevent from spamming
    (bind _result (Math|Integer|DecrementInt (Variables|Default|GetAmmo))
      (:%20%20
        (Variables|Default|SetAmmo _result)
        (Utilities|FlowControl|Delay 1.0)
        (Variables|Default|SetAmmo (Variables|Default|GetmaxAmmo))))))

(fn ConstructionScript
  (|CallParentFunction))