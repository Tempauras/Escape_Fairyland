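; Elemental gun weapon that switches between fire, water, wind and earth, firing the matching bullet class.
; Element input actions set a shared index that selects the bullet and recolors the gun through a dynamic material instance.
; EndShooting spawns the bullet along the camera rotation, offset by the first-person character's GunOffset, while BeginShooting is empty.
; A one-round magazine that refills after a short delay limits the fire rate.
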(event EventBeginPlay
  (bind _skeletalmesh (Variables|Default|GetSkeletalMesh))
  (Input|EnableInput (Game|GetPlayerController 0))
  (Variables|Default|SetColors (Utilities|Array|MakeArray (Variables|Default|GetFire) (Variables|Default|GetWater) (Variables|Default|GetWind) (Variables|Default|GetEarth)))
  (Variables|Default|SetBullets (Utilities|Array|MakeArray (Variables|Default|GetFireBullet) (Variables|Default|GetWaterBullet) (Variables|Default|GetWindBullet) (Variables|Default|GetEarthBullet)))
  (bind _returnvalue (Rendering|Material|CreateDynamicMaterialInstance _skeletalmesh 0 (Rendering|Material|GetMaterial _skeletalmesh 0) "None" :!class /Script/Engine.PrimitiveComponent))
  (bind _output_get (Variables|Default|SetMIWeapon _returnvalue))
  (Rendering|Material|SetVectorParameterValue _output_get "MasterPaintColour" (Variables|Default|GetFire) :!class /Script/Engine.MaterialInstanceDynamic)
  (bind _output_get_2 (Variables|Default|SetMaxAmmo 1))
  (Variables|Default|SetCurrentAmmo _output_get_2))

(event EventBeginShooting)

(event EventEndShooting
  (bind _returnvalue (Game|GetPlayerCameraManager 0))
  (bind _transformcomponent (Variables|/Script/Engine.PlayerCameraManager|GetTransformComponent _returnvalue))
  (bind _returnvalue_2 (Transformation|GetWorldRotation _transformcomponent))
  (if (> (Variables|Default|GetCurrentAmmo) 0)
    (Audio|PlaySound2D "/Game/FirstPerson/Audio/FirstPersonTemplateWeaponFire02.FirstPersonTemplateWeaponFire02" 1.0 1.0 0.0 0 0)
    (bind _asfirst_person_character (Utilities|Casting|CastToFirstPersonCharacter (Game|Player|GetPlayerPawn 0)))
    (Game|SpawnActorfromClass (Utilities|Array|Get(acopy) (Variables|Default|GetBullets) (Variables|Default|GetArrayIndex)) (Math|Transform|MakeTransform (+ (Math|Vector|RotateVector (Variables|/Game/FirstPersonBP/Blueprints/FirstPersonCharacter.FirstPersonCharacter_C|GetGunOffset _asfirst_person_character) _returnvalue_2) (Transformation|GetWorldLocation (Variables|Default|GetSkeletalMesh))) _returnvalue_2) "Undefined" 0 0)
    (bind _result (Math|Integer|DecrementInt (Variables|Default|GetCurrentAmmo))
      (:%20%20
        (Variables|Default|SetCurrentAmmo _result)
        (Utilities|FlowControl|Delay 0.5)
        (Variables|Default|SetCurrentAmmo (Variables|Default|GetMaxAmmo))))))

(event Input|ActionEvents|InputActionChangeToFire
  (params (Key :type Key%20Structure :default "None"))
  (:Pressed
    (bind _output_get (Variables|Default|SetArrayIndex 0))
    (CallFunction|ChangeElement _output_get)))

(event Input|ActionEvents|InputActionChangeToWater
  (params (Key :type Key%20Structure :default "None"))
  (:Pressed
    (bind _output_get (Variables|Default|SetArrayIndex 1))
    (CallFunction|ChangeElement _output_get)))

(event Input|ActionEvents|InputActionChangeToWind
  (params (Key :type Key%20Structure :default "None"))
  (:Pressed
    (bind _output_get (Variables|Default|SetArrayIndex 2))
    (CallFunction|ChangeElement _output_get)))

(event Input|ActionEvents|InputActionChangeToEarth
  (params (Key :type Key%20Structure :default "None"))
  (:Pressed
    (bind _output_get (Variables|Default|SetArrayIndex 3))
    (CallFunction|ChangeElement _output_get)))

(fn ConstructionScript
  (|CallParentFunction))

(fn ChangeElement
  (params (index :type Integer))
  (Rendering|Material|SetVectorParameterValue (Variables|Default|GetMIWeapon) "MasterPaintColour" (Utilities|Array|Get(acopy) (Variables|Default|GetColors) index) :!class /Script/Engine.MaterialInstanceDynamic))