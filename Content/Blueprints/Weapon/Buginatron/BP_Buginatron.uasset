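; Buginatron weapon, a child of a base weapon, that temporarily makes static meshes it hits intangible.
; Releasing fire traces toward the camera's aim, ignoring cacti, then disables the hit component's collision and applies a shield material to static mesh actors.
; A full charge extends the effect.
; After the delay it restores collision, materials and ammo, launching the player away if the box overlap taken at hit time found something.
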(event Custom|ChangeMaterial
  (params (A :type Boolean))
  (bind _asstatic_mesh_actor (Utilities|Casting|CastToStaticMeshActor (Variables|Default|GetHit%20Actor)))
  (if A
    (Variables|Default|SetoldMaterials (Rendering|Material|GetMaterials (Variables|/Script/Engine.StaticMeshActor|GetStaticMeshComponent _asstatic_mesh_actor)))
    (for (_ _array_index) (Rendering|Material|GetMaterials (Variables|/Script/Engine.StaticMeshActor|GetStaticMeshComponent _asstatic_mesh_actor))
      (Rendering|Material|SetMaterial (Variables|/Script/Engine.StaticMeshActor|GetStaticMeshComponent _asstatic_mesh_actor) _array_index "/Game/Blueprints/Weapon/Buginatron/MaterialLib/sphere_shield_Inst.sphere_shield_Inst"))
    (else
      (for (_ _array_index_2) (Rendering|Material|GetMaterials (Variables|/Script/Engine.StaticMeshActor|GetStaticMeshComponent _asstatic_mesh_actor))
        (Rendering|Material|SetMaterial (Variables|/Script/Engine.StaticMeshActor|GetStaticMeshComponent _asstatic_mesh_actor) _array_index_2 (Utilities|Array|Get(acopy) (Variables|Default|GetoldMaterials) _array_index_2))))))

(event EventTick
  (params (DeltaSeconds :type Float%20%28single-precision%29))
  (if (Variables|Default|GetisCharging)
    (Variables|Default|Setcharge (* (Class|PlayerController|GetInputKeyTimeDown (Game|GetPlayerController 0) "LeftMouseButton") 3.0))))

(event EventActivateUI
  (bind _returnvalue (UserInterface|CreateWidget "/Game/Blueprints/UI/WG_buginatron.WG_buginatron_C"))
  (UserInterface|Viewport|AddtoViewport _returnvalue 1)
  (bind _asfirst_person_character (Utilities|Casting|CastToFirstPersonCharacter (Game|GetPlayerCharacter 0)))
  (Variables|/Game/Blueprints/UI/WG_buginatron.WG_buginatron_C|Setplayer _returnvalue _asfirst_person_character))

(event EventEndShooting
  (bind _maxcharge (Variables|Default|GetmaxCharge))
  ;[1 1 1] Overrided Shooting Methods Base Weapon
  (Variables|Default|SetisCharging false)
  (if (> (Variables|Default|Getcharge) _maxcharge)
    (bind _output_get (Variables|Default|Setcharge _maxcharge))
    (Variables|Default|SetcurrPowerTime (+ _output_get (Variables|Default|GetcurrPowerTime))))
  (CallFunction|Shoot))

(event EventShoot
  (bind _returnvalue (Game|GetPlayerCameraManager 0))
  (bind _returnvalue_2 (Transformation|GetActorLocation _returnvalue))
  ;[1 1 1] TraceShot
  ;;[1 1 1] Test ammo
  (if (> (Variables|Default|Getammo) 0)
    (bind (_outhit _returnvalue_3) (Collision|LineTraceByChannel (Transformation|GetSocketLocation (Variables|Default|GetSkeletalMesh) "shotPoint") (+ _returnvalue_2 (* (Transformation|GetActorForwardVector _returnvalue) (Variables|Default|Getrange))) "TraceTypeQuery1" false (Variables|Default|GetActorsToIgnore) "None"))
    (if _returnvalue_3
      (Niagara|SpawnSystematLocation "/Game/ThirdParty/Stylized_VFX_StPack/Particles/UPDATE_1_2/P_CosmicHit_01.P_CosmicHit_01" (.Location (Collision|BreakHitResult _outhit)))
      (Audio|PlaySoundatLocation "/Game/Blueprints/Weapon/Buginatron/BLASTR.BLASTR" _returnvalue_2 "0, 0, 0" 1.0 1.0 0.0 0 0 0)
      (Variables|Default|Setammo (+ (Variables|Default|Getammo) -1))
      (Variables|Default|SetHit%20Actor (.HitActor (Collision|BreakHitResult _outhit)))
      ;[1 1 1] Make the object touch intangible
      (CallFunction|ChangeMaterial true)
      (bind _output_get (Variables|Default|SetHit%20Component (.HitComponent (Collision|BreakHitResult _outhit))))
      (Collision|SetCollisionProfileName _output_get "NoCollision" true :!class /Script/Engine.PrimitiveComponent)
      (bind _returnvalue_4 (Collision|BoxOverlapActors (.Origin (Collision|GetActorBounds (Variables|Default|GetHit%20Actor) false false)) (.BoxExtent (Collision|GetActorBounds (Variables|Default|GetHit%20Actor) false false)) (Variables|Default|GetobjectTypesBoxOverlap) 0 :!class /Script/Engine.KismetSystemLibrary))
      (Utilities|FlowControl|Delay (Variables|Default|GetcurrPowerTime))
      ;[1 1 1] Make the object tangible again
      (if _returnvalue_4
        (Character|LaunchCharacter (Game|GetPlayerCharacter 0) (* (* (Math|Vector|GetUnitDirection(Vector) (.Location (Collision|BreakHitResult _outhit)) (.TraceStart (Collision|BreakHitResult _outhit))) 5e+02) (Variables|Default|GetcurrPowerTime)) true true))
      (Collision|SetCollisionProfileName (Variables|Default|GetHit%20Component) "BlockAll" false :!class /Script/Engine.PrimitiveComponent)
      (CallFunction|ChangeMaterial false)
      (Variables|Default|Setammo (+ (Variables|Default|Getammo) 1))
      (Variables|Default|SetcurrPowerTime (Variables|Default|GetpowerTime))
      (Audio|PlaySoundatLocation "/Game/Blueprints/Weapon/Buginatron/SHRINK.SHRINK" _returnvalue_2 "0, 0, 0" 1.0 1.0 0.0 0 0 0))
    (else
      (Development|PrintString "NoAmmo"))))

(event EventBeginPlay
  ;[1 1 1] GetAllEnnemies
  (bind _outactors (Actor|GetAllActorsOfClass "/Game/Blueprints/Characters/Cactus/BP_Cactus.BP_Cactus_C"))
  (Variables|Default|SetActorsToIgnore _outactors))

(event EventBeginShooting
  ;[1 1 1] Overrided Shooting Methods Base Weapon
  (Variables|Default|SetisCharging true))

(fn ConstructionScript
  (|CallParentFunction))