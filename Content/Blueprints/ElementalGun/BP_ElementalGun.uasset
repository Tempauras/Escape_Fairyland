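; Elemental rifle weapon that switches between Fire, Water, Wind and Earth and fires the matching projectile class.
; Element input actions set a shared index into parallel color and bullet arrays, recoloring the weapon through a dynamic material instance.
; Shoot spawns the selected bullet at the mesh location with camera rotation, then refills the single-round ammo after a short delay, acting as a fire-rate limit.
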(event EventBeginPlay
  (bind _skeletalmesh (Variables|Default|GetSkeletalMesh))
  (Input|EnableInput (Game|GetPlayerController 0))
  (Variables|Default|SetColors (Utilities|Array|MakeArray (Variables|Default|GetFire) (Variables|Default|GetWater) (Variables|Default|GetWind) (Variables|Default|GetEarth)))
  (Variables|Default|SetBullets (Utilities|Array|MakeArray (Variables|Default|GetFireBullet) (Variables|Default|GetWaterBullet) (Variables|Default|GetWindBullet) (Variables|Default|GetEarthBullet)))
  (bind _returnvalue (Rendering|Material|CreateDynamicMaterialInstance _skeletalmesh 0 (Rendering|Material|GetMaterial _skeletalmesh 0) "None" :!class /Script/Engine.PrimitiveComponent))
  (bind _output_get (Variables|Default|SetMIWeapon _returnvalue))
  (Rendering|Material|SetVectorParameterValue _output_get "MasterPaintColour" (Variables|Default|GetFire) :!class /Script/Engine.MaterialInstanceDynamic)
  (bind _output_get_2 (Variables|Default|SetMaxAmmo 1))
  (Variables|Default|SetCurrentAmmo _output_get_2))

(event EventShoot
  (if (> (Variables|Default|GetCurrentAmmo) 0)
    (Development|PrintString "Elemental Rifle shoot")
    (Game|SpawnActorfromClass (Utilities|Array|Get(acopy) (Variables|Default|GetBullets) (Variables|Default|GetArrayIndex)) (Math|Transform|MakeTransform (Transformation|GetWorldLocation (Variables|Default|GetSkeletalMesh)) (Transformation|GetWorldRotation (Variables|/Script/Engine.PlayerCameraManager|GetTransformComponent (Game|GetPlayerCameraManager 0)))) "Undefined" 0 0)
    (bind _result (Math|Integer|DecrementInt (Variables|Default|GetCurrentAmmo))
      (:%20%20
        (Variables|Default|SetCurrentAmmo _result)
        (Utilities|FlowControl|Delay 0.5)
        (Variables|Default|SetCurrentAmmo (Variables|Default|GetMaxAmmo))))
    (else
      (Development|PrintString "Out Of Ammo!"))))

(event Input|ActionEvents|InputActionChangeToFire
  (params (Key :type Key%20Structure :default "None"))
  (:Pressed
    (bind _output_get (Variables|Default|SetArrayIndex 0))
    (CallFunction|ChangeElement _output_get)))

(event Input|ActionEvents|InputActionChangeToWater
  (params (Key :type Key%20Structure :default "None"))
  (:Pressed
    (bind _output_get (Variables|Default|SetArrayIndex 1))
    (CallFunction|ChangeElement _output_get)))

(event Input|ActionEvents|InputActionChangeToWind
  (params (Key :type Key%20Structure :default "None"))
  (:Pressed
    (bind _output_get (Variables|Default|SetArrayIndex 2))
    (CallFunction|ChangeElement _output_get)))

(event Input|ActionEvents|InputActionChangeToEarth
  (params (Key :type Key%20Structure :default "None"))
  (:Pressed
    (bind _output_get (Variables|Default|SetArrayIndex 3))
    (CallFunction|ChangeElement _output_get)))

(fn ConstructionScript
  (|CallParentFunction))

(fn ChangeElement
  (params (Dimension%201 :type Integer))
  (Rendering|Material|SetVectorParameterValue (Variables|Default|GetMIWeapon) "MasterPaintColour" (Utilities|Array|Get(acopy) (Variables|Default|GetColors) Dimension%201) :!class /Script/Engine.MaterialInstanceDynamic))