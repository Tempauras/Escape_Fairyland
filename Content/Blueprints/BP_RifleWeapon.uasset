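; BP_RifleWeapon is a rifle weapon Blueprint that fires a hitscan shot when its Shoot event is called.
; Shoot prints a debug message, then line-traces on the Visibility channel from the first player's camera manager along its forward vector for a fixed range.
; On a hit it spawns a tutorial particle emitter at the impact point, with no damage applied.
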(event EventBeginPlay
  (|CallParentFunction) ; This node is disabled and will not be called.\nDrag off pins to build functionality.
)

(event Collision|EventActorBeginOverlap
  (params (OtherActor :type Actor%20Object%20Reference))
  (|CallParentFunction OtherActor) ; This node is disabled and will not be called.\nDrag off pins to build functionality.
)

(event EventTick
  (params (DeltaSeconds :type Float%20%28single-precision%29))
  (|CallParentFunction DeltaSeconds) ; This node is disabled and will not be called.\nDrag off pins to build functionality.
)

(event EventShoot
  (bind _returnvalue (Game|GetPlayerCameraManager 0))
  (bind _returnvalue_2 (Transformation|GetActorLocation _returnvalue))
  (Development|PrintString "Rifle Weapon Shoot" true true "(R=0.843933,G=1.000000,B=0.304575,A=1.000000)")
  (bind (_outhit _returnvalue_3) (Collision|LineTraceByChannel _returnvalue_2 (+ _returnvalue_2 (* (Transformation|GetActorForwardVector _returnvalue) 5e+03)) "TraceTypeQuery1" false 0 "None"))
  (if _returnvalue_3
    (Effects|SpawnEmitteratLocation "/Engine/Tutorial/SubEditors/TutorialAssets/TutorialParticleSystem.TutorialParticleSystem" (.ImpactPoint (Collision|BreakHitResult _outhit)))))

(fn ConstructionScript
  (|CallParentFunction))