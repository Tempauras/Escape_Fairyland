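; BP_FanMultiDrifting is a fan prop that switches on, along with every other instance, when a WindBullet hits its Box.
; The hit, gated by a DoOnce, calls CallEDMoveCloudLoop, then starts each fan's animation and disables its Box collision.
; A timeline drives each fan's Spinning component through local pitch rotation.
; A switch-on sound plays at a hardcoded world location, followed after a delay by a loop sound.
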(event OnComponentHit(Box)
  (params (HitComponent :type Primitive%20Component%20Object%20Reference) (OtherActor :type Actor%20Object%20Reference) (OtherComp :type Primitive%20Component%20Object%20Reference) (NormalImpulse :type Vector :default "0, 0, 0") (Hit :type Hit%20Result%20Structure%20%28by%20ref%29))
  (bind _returnvalue (Math|Vector|MakeVector 6.23e+03 -1.137e+04 1.2e+03))
  (Utilities|FlowControl|DoOnce false
    (:Completed
      (if (== (Utilities|GetClass OtherActor) "/Game/Blueprints/Weapon/ElementalGun/BP/WindBullet.WindBullet_C")
        (Default|CallEDMoveCloudLoop)
        (bind _outactors (Actor|GetAllActorsOfClass "BP_FanMultiDrifting_C"))
        (for _array_element _outactors
          (CallFunction|StartFanAnimation _array_element)
          (Collision|SetCollisionEnabled (Variables|BP_FanMultiDrifting_C|GetBox _array_element) "NoCollision"))
        (Audio|PlaySoundatLocation "/Game/ThirdParty/Sounds/SoundEffect/Fan_Sound_on.Fan_Sound_on" _returnvalue "0, 0, 0" 1.0 1.0 0.0 0 0 0)
        (Utilities|FlowControl|Delay 3.9)
        (Audio|PlaySoundatLocation "/Game/ThirdParty/Sounds/SoundEffect/Fan_Sound_Loop.Fan_Sound_Loop" _returnvalue "0, 0, 0" 1.0 1.0 0.0 0 0 0)))))

(event Custom|StartFanAnimation
  (bind _y__pitch_ (Timeline|FanAnimationTimeline Play)
    (:Update
      (Transformation|AddLocalRotation (Variables|Default|GetSpinning) (Math|Rotator|MakeRotator 0.0 _y__pitch_ 0.0) false false))))

(event EventBeginPlay)

(event Collision|EventActorBeginOverlap
  (params (OtherActor :type Actor%20Object%20Reference)))

(fn ConstructionScript)