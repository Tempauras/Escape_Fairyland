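; Fire wall prop that hurts the player on contact and can be put out with water bullets.
; On mesh hit, after a short delay, each WaterBullet lowers the wall's life until it is destroyed.
; A FirstPersonCharacter hit instead receives damage through UpdateLife and is launched using the impact normal for X and Z, with a fixed strong push along world Y.
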(event OnComponentHit(StaticMeshComponent)
  (params (HitComponent :type Primitive%20Component%20Object%20Reference) (OtherActor :type Actor%20Object%20Reference) (OtherComp :type Primitive%20Component%20Object%20Reference) (NormalImpulse :type Vector :default "0, 0, 0") (Hit :type Hit%20Result%20Structure%20%28by%20ref%29))
  (bind _returnvalue (Utilities|GetClass OtherActor))
  (bind _impactnormal (Collision|BreakHitResult Hit))
  (bind _returnvalue_2 (* _impactnormal 3e+02))
  (bind (_x _y _z) (Math|Vector|BreakVector _returnvalue_2))
  (Utilities|FlowControl|Delay 0.1)
  (if (== _returnvalue "/Game/Blueprints/Weapon/ElementalGun/BP/WaterBullet.WaterBullet_C")
    (bind _result (Math|Float|DecrementFloat (Variables|Default|GetcurrentLife))
      (:%20%20
        (if (<= _result 0.0)
          (Actor|DestroyActor))))
    (elif (== _returnvalue "/Game/FirstPersonBP/Blueprints/FirstPersonCharacter.FirstPersonCharacter_C")
      (bind _asfirst_person_character (Utilities|Casting|CastToFirstPersonCharacter OtherActor))
      (Default|UpdateLife _asfirst_person_character (Variables|Default|GetcontactDamage))
      (Character|LaunchCharacter _asfirst_person_character (Math|Vector|MakeVector _x 2.5e+03 _z) false false))))

(event EventBeginPlay
  (Variables|Default|SetcontactDamage -1e+01)
  (bind _output_get (Variables|Default|SetmaxLife 4.0))
  (Variables|Default|SetcurrentLife _output_get))

(fn ConstructionScript)