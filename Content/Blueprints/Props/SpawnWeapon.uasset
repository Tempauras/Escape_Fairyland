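; SpawnWeapon is a prop that displays a weapon and gives it to the player on contact.
; On BeginPlay it caches the player character and spawns an actor of its Weapon class slightly above itself.
; When the player overlaps its Sphere, it passes that class to FirstPersonCharacter's SwitchWeapon, sets the equipped index and updates the equipped weapon.
; The prop never removes itself or the spawned actor.
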(event OnComponentBeginOverlap(Sphere)
  (params (OverlappedComponent :type Primitive%20Component%20Object%20Reference) (OtherActor :type Actor%20Object%20Reference) (OtherComp :type Primitive%20Component%20Object%20Reference) (OtherBodyIndex :type Integer) (bFromSweep :type Boolean) (SweepResult :type Hit%20Result%20Structure%20%28by%20ref%29))
  (bind _player (Variables|Default|Getplayer))
  (if (== OtherActor _player)
    (bind _asfirst_person_character (Utilities|Casting|CastToFirstPersonCharacter _player))
    (Default|SwitchWeapon _asfirst_person_character (Variables|Default|Getweapon))
    (Variables|/Game/FirstPersonBP/Blueprints/FirstPersonCharacter.FirstPersonCharacter_C|SetWeaponEquippedIndex _asfirst_person_character 1)
    (Default|UpdateEquippedWeapon _asfirst_person_character)))

(event EventBeginPlay
  (bind _returnvalue (Transformation|GetActorTransform))
  (Variables|Default|Setplayer (Game|GetPlayerCharacter 0))
  (Game|SpawnActorfromClass (Variables|Default|Getweapon) (Math|Transform|MakeTransform (+ (.location _returnvalue) (Math|Vector|MakeVector 0.0 0.0 1e+02)) (.rotation _returnvalue) (.scale _returnvalue)) "Undefined" 0 0))

(fn ConstructionScript)