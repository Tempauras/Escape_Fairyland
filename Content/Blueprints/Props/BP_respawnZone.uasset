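; BP_respawnZone is a prop trigger box that handles the player or cacti entering it.
; When the player pawn overlaps the box, it asks BP_GameMode to respawn the player, then calls UpdateLife on the player's FirstPersonCharacter with a negative amount as a penalty.
; Any overlapping BP_Cactus is told to Die, and other actors are ignored.
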(event OnComponentBeginOverlap(Box)
  (params (OverlappedComponent :type Primitive%20Component%20Object%20Reference) (OtherActor :type Actor%20Object%20Reference) (OtherComp :type Primitive%20Component%20Object%20Reference) (OtherBodyIndex :type Integer) (bFromSweep :type Boolean) (SweepResult :type Hit%20Result%20Structure%20%28by%20ref%29))
  (bind _returnvalue (Game|Player|GetPlayerPawn 0))
  (if (== OtherActor _returnvalue)
    (bind _asbp_game_mode (Utilities|Casting|CastToBP_GameMode (Game|GetGameMode)))
    (Default|RespawnPlayer _asbp_game_mode)
    (bind _asfirst_person_character (Utilities|Casting|CastToFirstPersonCharacter _returnvalue))
    (Default|UpdateLife _asfirst_person_character -3e+01)
    (elif (== (Utilities|GetClass OtherActor) "/Game/Blueprints/Characters/Cactus/BP_Cactus.BP_Cactus_C")
      (bind _asbp_cactus (Utilities|Casting|CastToBP_Cactus OtherActor))
      (Default|Die _asbp_cactus))))

(fn ConstructionScript)