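; BP_PushableCrate is a prop crate that gets pushed when an EarthBullet hits it.
; On a mesh hit from an EarthBullet, it applies an impulse along the bullet's forward vector.
; It stores its transform at BeginPlay, and a ResetPosition event teleports the mesh back to that spawn transform.
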(event OnComponentHit(StaticMeshComponent)
  (params (HitComponent :type Primitive%20Component%20Object%20Reference) (OtherActor :type Actor%20Object%20Reference) (OtherComp :type Primitive%20Component%20Object%20Reference) (NormalImpulse :type Vector :default "0, 0, 0") (Hit :type Hit%20Result%20Structure%20%28by%20ref%29))
  (if (== (Utilities|GetClass OtherActor) "/Game/Blueprints/Weapon/ElementalGun/BP/EarthBullet.EarthBullet_C")
    (Physics|AddImpulse (Variables|Debug|GetStaticMeshComponent) (* (Transformation|GetActorForwardVector OtherActor) 1e+03) "None" false)))

(event Custom|ResetPosition
  (Transformation|SetWorldTransform (Variables|Debug|GetStaticMeshComponent) (Variables|Default|GetspawnTransform) false true))

(event EventBeginPlay
  (Variables|Default|SetspawnTransform (Transformation|GetActorTransform)))

(fn ConstructionScript)