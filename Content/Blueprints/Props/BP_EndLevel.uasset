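; BP_EndLevel is a spinning level-exit prop that sends the player to the next level on touch.
; Tick adds RotationSpeed scaled by delta time to its yaw each frame.
; When the player pawn overlaps its Sphere component, it casts the game mode to BP_GameMode and calls NextLevel.
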(event OnComponentBeginOverlap(Sphere)
  (params (OverlappedComponent :type Primitive%20Component%20Object%20Reference) (OtherActor :type Actor%20Object%20Reference) (OtherComp :type Primitive%20Component%20Object%20Reference) (OtherBodyIndex :type Integer) (bFromSweep :type Boolean) (SweepResult :type Hit%20Result%20Structure%20%28by%20ref%29))
  (if (== OtherActor (Game|Player|GetPlayerPawn 0))
    (bind _asbp_game_mode (Utilities|Casting|CastToBP_GameMode (Game|GetGameMode)))
    (Default|NextLevel _asbp_game_mode)))

(event EventTick
  (params (DeltaSeconds :type Float%20%28single-precision%29))
  (bind _returnvalue (Transformation|GetActorRotation))
  (Transformation|SetActorRotation (Math|Rotator|MakeRotator (.roll _returnvalue) (.pitch _returnvalue) (+ (* DeltaSeconds (Variables|Default|GetrotationSpeed)) (.yaw _returnvalue)))))

(fn ConstructionScript)