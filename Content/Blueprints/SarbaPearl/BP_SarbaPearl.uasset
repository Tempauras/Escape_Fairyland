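; BP_SarbaPearl is an ammo-limited shooter that fires BP_SarbaBullet actors.
; The Releasing event calls Shoot, which, if ammo remains, spawns a bullet just ahead of the Arrow component along its facing and decrements Ammo.
; A one-second Delay then restores Ammo to MaxAmmo, the value it also receives on BeginPlay.
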(event EventBeginPlay
  (Variables|Default|SetAmmo (Variables|Default|GetmaxAmmo)))

(event EventReleasing
  (CallFunction|Shoot))

(event EventShoot
  (bind _arrow (Variables|Default|GetArrow))
  (if (> (Variables|Default|GetAmmo) 0)
    (Game|SpawnActorfromClass "/Game/Blueprints/SarbaPearl/BP_SarbaBullet.BP_SarbaBullet_C" (Math|Transform|MakeTransform (+ (Transformation|GetWorldLocation _arrow) (Math|Vector|GetForwardVector _arrow)) (Transformation|GetWorldRotation _arrow) "1,1,1") "AdjustIfPossibleButAlwaysSpawn" 0 5e+02 0)
    (bind _result (Math|Integer|DecrementInt (Variables|Default|GetAmmo))
      (:%20%20
        (Variables|Default|SetAmmo _result)
        (Utilities|FlowControl|Delay 1.0)
        (Variables|Default|SetAmmo (Variables|Default|GetmaxAmmo))))))

(fn ConstructionScript
  (|CallParentFunction))