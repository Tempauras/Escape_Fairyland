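; BP_Cactus is an AI cactus enemy that spots the player, shoots projectiles and can be stunned or killed.
; A detection sphere writes player sight and the target actor to the Blackboard while it is alive.
; CactusShoot fires a projectile aimed midway between the player and camera positions, then re-allows movement.
; Radial damage lowers clamped health and briefly stops it with a hit animation; death flags the AnimBP and detaches the controller.
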(event OnComponentBeginOverlap(DetectionSphere)
  (params (OverlappedComponent :type Primitive%20Component%20Object%20Reference) (OtherActor :type Actor%20Object%20Reference) (OtherComp :type Primitive%20Component%20Object%20Reference) (OtherBodyIndex :type Integer) (bFromSweep :type Boolean) (SweepResult :type Hit%20Result%20Structure%20%28by%20ref%29))
  (bind _blackboardref (Variables|Default|GetBlackBoardRef))
  ;[1 1 1] PlayerDetection
  (if (Math|Boolean|Equal(Boolean) (Variables|Default|GetisDead) false)
    (if (Actor|ActorHasTag OtherActor "Player")
      (AI|Components|Blackboard|SetValueasBool _blackboardref (Variables|Default|GetOnSight) true)
      (AI|Components|Blackboard|SetValueasObject _blackboardref (Variables|Default|GetEnnemyActor) OtherActor))))

(event OnComponentEndOverlap(DetectionSphere)
  (params (OverlappedComponent :type Primitive%20Component%20Object%20Reference) (OtherActor :type Actor%20Object%20Reference) (OtherComp :type Primitive%20Component%20Object%20Reference) (OtherBodyIndex :type Integer))
  ;[1 1 1] PlayerDetection
  (if (Math|Boolean|Equal(Boolean) (Variables|Default|GetisDead) false)
    (if (Actor|ActorHasTag OtherActor "Player")
      (AI|Components|Blackboard|SetValueasBool (Variables|Default|GetBlackBoardRef) (Variables|Default|GetOnSight) false))))

(event Custom|Die
  (Variables|Default|SetisDead true)
  (bind _asabp_cactus (Utilities|Casting|CastToABP_Cactus (Components|SkeletalMesh|GetAnimInstance (Variables|Character|GetMesh))))
  (Variables|/Game/Blueprints/Characters/Cactus/ABP_Cactus.ABP_Cactus_C|SetisDead _asabp_cactus true)
  (Development|PrintString "Cactus Die")
  (Class|Pawn|DetachfromControllerPendingDestroy))

(event Custom|CactusShoot
  (bind _returnvalue (Transformation|GetActorTransform))
  ;[1 1 1] SpawnProjectile
  (Game|SpawnActorfromClass "/Game/Blueprints/Characters/Cactus/BP_CactusProjectile.BP_CactusProjectile_C" (Math|Transform|MakeTransform (.location _returnvalue) (Math|Rotator|FindLookatRotation (.location _returnvalue) (/ (+ (Transformation|GetActorLocation (Variables|Default|GetPlayerRef)) (Camera|GetCameraLocation (Variables|Default|GetCameraRef))) 2.0)) "1,1,1") "AlwaysSpawn" 0 0)
  (AI|Components|Blackboard|SetValueasBool (Variables|Default|GetBlackBoardRef) (Variables|Default|GetAllowMove) true))

(event Game|Damage|EventRadialDamage
  (params (DamageReceived :type Float%20%28single-precision%29) (DamageType :type Damage%20Type%20Object%20Reference) (Origin :type Vector :default "0, 0, 0") (HitInfo :type Hit%20Result%20Structure%20%28by%20ref%29) (InstigatedBy :type Controller%20Object%20Reference) (DamageCauser :type Actor%20Object%20Reference))
  (bind _asabp_cactus (Utilities|Casting|CastToABP_Cactus (Components|SkeletalMesh|GetAnimInstance (Variables|Character|GetMesh))))
  (Variables|/Game/Blueprints/Characters/Cactus/ABP_Cactus.ABP_Cactus_C|SetisHit _asabp_cactus true)
  (Components|Movement|StopMovementImmediately (Variables|Character|GetCharacterMovement))
  (CallFunction|UpdateHealth (* DamageReceived -1.0))
  (Utilities|FlowControl|Delay (Variables|Default|GetstunTime))
  (Variables|/Game/Blueprints/Characters/Cactus/ABP_Cactus.ABP_Cactus_C|SetisHit _asabp_cactus false)
  (Development|PrintString (Utilities|String|ToString(Float) (Variables|Default|GetHealth))))

(event EventBeginPlay
  (Variables|Default|SetBlackBoardRef (AI|GetBlackboard self))
  (Variables|Default|SetPlayerRef (Game|Player|GetPlayerPawn 0))
  (Variables|Default|SetCameraRef (Game|GetPlayerCameraManager 0)))

(fn ConstructionScript)

(fn UpdateHealth
  (params (addHealth :type Float%20%28single-precision%29))
  (bind _maxhealth (Variables|Default|GetMaxHealth))
  (if (<= (+ addHealth (Variables|Default|GetHealth)) 0.0)
    (CallFunction|Die)
    (elif (>= (+ addHealth (Variables|Default|GetHealth)) _maxhealth)
      (Variables|Default|SetHealth _maxhealth)
      (else
        (Variables|Default|SetHealth (+ addHealth (Variables|Default|GetHealth)))))))