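; BP_Torches is a torch actor that lights when a FireBullet hits its Box component.
; On that hit it calls the TorchIsLit event dispatcher and swaps the Fire component's material to the torch toon-fire instance.
; It then creates a fresh dynamic material instance, and SpawnTimeline drives its Strength parameter to animate the flame appearing.
; BeginPlay also creates a dynamic instance from the starting material.
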(event OnComponentHit(Box)
  (params (HitComponent :type Primitive%20Component%20Object%20Reference) (OtherActor :type Actor%20Object%20Reference) (OtherComp :type Primitive%20Component%20Object%20Reference) (NormalImpulse :type Vector :default "0, 0, 0") (Hit :type Hit%20Result%20Structure%20%28by%20ref%29))
  (bind _fire (Variables|Default|GetFire))
  (if (== (Utilities|GetClass OtherActor) "/Game/Blueprints/ElementalGun/BP/FireBullet.FireBullet_C")
    (Default|CallEDTorchIsLit)
    (Rendering|Material|SetMaterial _fire 0 "/Game/Blueprints/ElementalGun/Material/Fire/M_ToonFire_Inst_Torches.M_ToonFire_Inst_Torches")
    (bind _returnvalue (Rendering|Material|CreateDynamicMaterialInstance _fire 0 (Rendering|Material|GetMaterial _fire 0) "None" :!class /Script/Engine.PrimitiveComponent))
    (Variables|Default|SetMI_Fire _returnvalue)
    (bind _firewall_appearing_track (Timeline|SpawnTimeline Play)
      (:Update
        (Rendering|Material|SetScalarParameterValue (Variables|Default|GetMI_Fire) "Strength" _firewall_appearing_track :!class /Script/Engine.MaterialInstanceDynamic)))))

(event EventBeginPlay
  (bind _fire (Variables|Default|GetFire))
  (bind _returnvalue (Rendering|Material|GetMaterial _fire 0))
  (Variables|Default|SetFireMaterial _returnvalue)
  (bind _returnvalue_2 (Rendering|Material|CreateDynamicMaterialInstance _fire 0 _returnvalue "None" :!class /Script/Engine.PrimitiveComponent))
  (Variables|Default|SetMI_Fire _returnvalue_2))

(fn ConstructionScript)