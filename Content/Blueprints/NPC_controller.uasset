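; NPC controller that sends an NPC around the level toward coin actors it can reach.
; On BeginPlay it gathers all Pl_Coin_01 actors, keeping those whose location projects onto the navmesh in a ReachableCoins list.
; It moves to the last coin in the list, and a custom event removes a given coin and, if it was listed, moves on to the next.
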(event Custom|GoToNextCoin
  (bind _reachablecoins (Variables|Default|GetReachableCoins))
  (if (> (Utilities|Array|Length _reachablecoins) 0)
    (AI|Navigation|MovetoActor (Utilities|Array|Get(acopy) _reachablecoins (Utilities|Array|LastIndex _reachablecoins)) -1.0 true true true 0)))

(event Custom|CustomEvent_0
  (params (Coin :type Pl%20Coin%2001%20Object%20Reference))
  (bind _returnvalue (Utilities|Array|RemoveItem (Variables|Default|GetReachableCoins) Coin))
  (if _returnvalue
    (CallFunction|GotoNextCoin)))

(event EventBeginPlay
  (bind _outactors (Actor|GetAllActorsOfClass "/Game/ThirdParty/Platformer/Blueprints/Pl_Coin_01.Pl_Coin_01_C"))
  (for _array_element _outactors
    (if (.ReturnValue (AI|Navigation|ProjectPointtoNavigation (Transformation|GetActorLocation _array_element) 0 0 "0, 0, 0"))
      (Utilities|Array|AddUnique (Variables|Default|GetReachableCoins) _array_element)))
  (CallFunction|GotoNextCoin))

(fn ConstructionScript)