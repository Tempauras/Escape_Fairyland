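; BP_SarbaPearl is a teleport ability that moves the player pawn to the point being aimed at.
; Shoot line-traces on Visibility from the camera manager along its forward vector for Range, with one-frame debug drawing.
; On a hit, it waits a second, then teleports player 0's pawn to the impact point using this actor's rotation.
; A longer trailing Delay has nothing wired after it.
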(event EventBeginPlay)

(event Collision|EventActorBeginOverlap
  (params (OtherActor :type Actor%20Object%20Reference)))

(event EventTick
  (params (DeltaSeconds :type Float%20%28single-precision%29)))

(event EventShoot
  (bind _returnvalue (Game|GetPlayerCameraManager 0))
  (bind _returnvalue_2 (Transformation|GetActorLocation _returnvalue))
  (bind (_outhit _returnvalue_3) (Collision|LineTraceByChannel _returnvalue_2 (+ _returnvalue_2 (* (Transformation|GetActorForwardVector _returnvalue) (Variables|Default|GetRange))) "TraceTypeQuery1" false 0 "ForOneFrame"))
  (if _returnvalue_3
    (Utilities|FlowControl|Delay 1.0)
    (Transformation|Teleport (Game|Player|GetPlayerPawn 0) (.ImpactPoint (Collision|BreakHitResult _outhit)) (.rotation (Transformation|GetActorTransform)))
    (Utilities|FlowControl|Delay 1e+01)))

(fn ConstructionScript
  (|CallParentFunction))