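; Base weapon Blueprint that provides automatic fire of the first-person template projectile.
; beginShooting fires once immediately and starts a looping FireRate timer on baseWeaponShoot, which endShooting clears.
; Each shot spawns a projectile at the mesh's Ammo socket, aimed by player camera 0's rotation, and plays a fire sound.
; The Shoot event is empty, and the charge and release debug logic is disconnected.
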(event Custom|Shoot)

(event Custom|beginShooting
  (Development|PrintString "Base Weapon Shoot!")
  (CallFunction|BaseWeaponShoot)
  (bind _returnvalue (Utilities|Time|SetTimerbyFunctionName 0 "baseWeaponShoot" (Variables|Default|GetfireRate) true))
  (Variables|Default|SetgunTimer _returnvalue))

(event Custom|endShooting
  (Utilities|Time|ClearandInvalidateTimerbyHandle (Variables|Default|GetgunTimer)))

(fn ConstructionScript)

(fn BaseWeaponShoot
  (Game|SpawnActorfromClass "/Game/FirstPersonBP/Blueprints/FirstPersonProjectile.FirstPersonProjectile_C" (Math|Transform|MakeTransform (Transformation|GetSocketLocation (Variables|Default|GetSkeletalMesh) "Ammo") (Transformation|GetActorRotation (Game|GetPlayerCameraManager 0)) "1,1,1") "Undefined" 0 0)
  (Audio|PlaySoundatLocation "/Game/FirstPerson/Audio/FirstPersonTemplateWeaponFire02.FirstPersonTemplateWeaponFire02" (Transformation|GetActorLocation) "0, 0, 0" 1.0 1.0 0.0 0 0 0))