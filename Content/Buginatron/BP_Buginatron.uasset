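; Buginatron is a chargeable gun that temporarily disables collision on whatever component its shot hits.
; Holding fire builds Charge, which extends the effect only when it exceeds MaxCharge and gets clamped.
; A camera-aimed trace from the muzzle, ignoring cacti, spends ammo and removes collision for CurrPowerTime.
; Afterward, a box overlap on the target's bounds launches the player back toward the shot origin, then collision and ammo are restored.
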(event EventTick
  (params (DeltaSeconds :type Float%20%28single-precision%29))
  (if (Variables|Default|GetisCharging)
    (Development|PrintString "charging")
    (bind _output_get (Variables|Default|Setcharge (* (Class|PlayerController|GetInputKeyTimeDown (Game|GetPlayerController 0) "LeftMouseButton") 3.0)))
    (Development|PrintString (Utilities|String|ToString(Float) _output_get))))

(event EventEndShooting
  (bind _maxcharge (Variables|Default|GetmaxCharge))
  (Variables|Default|SetisCharging false)
  (if (> (Variables|Default|Getcharge) _maxcharge)
    (bind _output_get (Variables|Default|Setcharge _maxcharge))
    (Variables|Default|SetcurrPowerTime (+ _output_get (Variables|Default|GetcurrPowerTime))))
  (CallFunction|Shoot))

(event EventShoot
  (bind _returnvalue (Game|GetPlayerCameraManager 0))
  (bind _returnvalue_2 (Transformation|GetActorLocation _returnvalue))
  ;[1 1 1] TraceShot
  ;;[1 1 1] Test ammo
  (if (> (Variables|Default|Getammo) 0)
    (bind (_outhit _returnvalue_3) (Collision|LineTraceByChannel (Transformation|GetSocketLocation (Variables|Default|GetSkeletalMesh) "shotPoint") (+ _returnvalue_2 (* (Transformation|GetActorForwardVector _returnvalue) (Variables|Default|Getrange))) "TraceTypeQuery1" false (Variables|Default|GetActorsToIgnore) "ForDuration"))
    (if _returnvalue_3
      (Audio|PlaySoundatLocation "/Game/FirstPerson/Audio/FirstPersonTemplateWeaponFire02.FirstPersonTemplateWeaponFire02" _returnvalue_2 "0, 0, 0" 1.0 1.0 0.0 0 0 0)
      (Variables|Default|Setammo (+ (Variables|Default|Getammo) -1))
      (Variables|Default|SetHit%20Actor (.HitActor (Collision|BreakHitResult _outhit)))
      (bind _output_get (Variables|Default|SetHit%20Component (.HitComponent (Collision|BreakHitResult _outhit))))
      (Collision|SetCollisionProfileName _output_get "NoCollision" true :!class /Script/Engine.PrimitiveComponent)
      (Utilities|FlowControl|Delay (Variables|Default|GetcurrPowerTime))
      (bind _returnvalue_4 (Collision|BoxOverlapActors (.Origin (Collision|GetActorBounds (Variables|Default|GetHit%20Actor) false false)) (.BoxExtent (Collision|GetActorBounds (Variables|Default|GetHit%20Actor) false false)) (Variables|Default|GetobjectTypesBoxOverlap) 0 :!class /Script/Engine.KismetSystemLibrary))
      (if _returnvalue_4
        (Character|LaunchCharacter (Game|GetPlayerCharacter 0) (* (* (Math|Vector|GetUnitDirection(Vector) (.Location (Collision|BreakHitResult _outhit)) (.TraceStart (Collision|BreakHitResult _outhit))) 5e+02) (Variables|Default|GetcurrPowerTime)) true true))
      (Collision|SetCollisionProfileName (Variables|Default|GetHit%20Component) "BlockAll" false :!class /Script/Engine.PrimitiveComponent)
      (Variables|Default|Setammo (+ (Variables|Default|Getammo) 1))
      (Variables|Default|SetcurrPowerTime (Variables|Default|GetpowerTime)))
    (else
      (Development|PrintString "NoAmmo"))))

(event EventBeginPlay
  (Variables|Default|SetcurrPowerTime (Variables|Default|GetpowerTime))
  (bind _outactors (Actor|GetAllActorsOfClass "/Game/Blueprints/Characters/Cactus/BP_Cactus.BP_Cactus_C"))
  (Variables|Default|SetActorsToIgnore _outactors))

(event EventBeginShooting
  (Variables|Default|SetisCharging true))

(fn ConstructionScript
  (|CallParentFunction))